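; Base target actor that feeds its Box's world location and extent into the materials of its visual components, with no runtime logic.
; The construction script rebuilds DynamicMaterials from Center's direct children, replacing static and skeletal mesh materials with dynamic instances.
; Niagara children receive an M_Particle instance through the MI_Niagara variable via SetNiagaraDynamicMaterial.
; Every instance gets Location and BoxExtent parameters, set only at construction.
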(fn `SetNiagaraDynamicMaterial`
  (params (Location :type "LinearColor Structure") (BoxExtent :type "LinearColor Structure") (NS_ParticleComp :type "NiagaraComponent Object Reference"))
  (bind _returnvalue (`KismetMaterialLibrary.CreateDynamicMaterialInstance` "/Game/Materials/M_Particle.M_Particle"))
  (`KismetArrayLibrary.Array_Add` (`self.DynamicMaterials`) _returnvalue)
  (`NiagaraComponent.SetVariableMaterial` NS_ParticleComp "MI_Niagara" _returnvalue)
  (`MaterialInstanceDynamic.SetVectorParameterValue` _returnvalue "Location" Location)
  (`MaterialInstanceDynamic.SetVectorParameterValue` _returnvalue "BoxExtent" BoxExtent))

(fn `UserConstructionScript`
  (bind _box (`self.Box`))
  (bind _returnvalue (`KismetMathLibrary.Conv_VectorToLinearColor` (`BoxComponent.BoxExtent` _box)))
  (bind _returnvalue_2 (`KismetMathLibrary.Conv_VectorToLinearColor` (`SceneComponent.K2_GetComponentLocation` _box)))
  (`KismetArrayLibrary.Array_Clear` (`self.DynamicMaterials`))
  (for _array_element (`SceneComponent.GetChildrenComponents` (`self.center`) false)
    (bind _asstatic_mesh_component (cast `StaticMeshComponent` _array_element)
      (:`then`
        (for (_array_element_2 _array_index) (`MeshComponent.GetMaterials` _asstatic_mesh_component)
          (bind _returnvalue_3 (`KismetMaterialLibrary.CreateDynamicMaterialInstance` _array_element_2))
          (`KismetArrayLibrary.Array_Add` (`self.DynamicMaterials`) _returnvalue_3)
          (`PrimitiveComponent.SetMaterial` _asstatic_mesh_component _array_index _returnvalue_3)
          (`MaterialInstanceDynamic.SetVectorParameterValue` _returnvalue_3 "Location" _returnvalue_2)
          (`MaterialInstanceDynamic.SetVectorParameterValue` _returnvalue_3 "BoxExtent" _returnvalue)))
      (:`CastFailed`
        (bind _asskeletal_mesh_component (cast `SkeletalMeshComponent` _array_element)
          (:`then`
            (for (_array_element_3 _array_index_2) (`MeshComponent.GetMaterials` _asskeletal_mesh_component)
              (bind _returnvalue_4 (`KismetMaterialLibrary.CreateDynamicMaterialInstance` _array_element_3))
              (`KismetArrayLibrary.Array_Add` (`self.DynamicMaterials`) _returnvalue_4)
              (`PrimitiveComponent.SetMaterial` _asskeletal_mesh_component _array_index_2 _returnvalue_4)
              (`MaterialInstanceDynamic.SetVectorParameterValue` _returnvalue_4 "Location" _returnvalue_2)
              (`MaterialInstanceDynamic.SetVectorParameterValue` _returnvalue_4 "BoxExtent" _returnvalue)))
          (:`CastFailed`
            (bind _asniagara_particle_system_component (cast `NiagaraComponent` _array_element))
            (`self.SetNiagaraDynamicMaterial` _returnvalue_2 _returnvalue _asniagara_particle_system_component)))))))