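; Slice capture actor that renders the scene as a row of orthographic depth slices and registers each for Spout output.
; Each slice gets a scene capture offset along local X, its own render target, and a post-process material instance with depth range spanning one interval.
; Render targets pair with Spout outputs in the Media Capture panel.
; Construction Script and BeginPlay duplicate this teardown and rebuild; neither starts capture.
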(event `self.ReceiveBeginPlay`
  (`|ExecutionSequence`
    (:`then_0`
      (for _array_element (`self.SceneCapture2DComponents`)
        (`ActorComponent.K2_DestroyComponent` _array_element null)))
    (:`then_1`
      (bind _returnvalue (`MediaFrameworkCapturePanelBlueprintLibrary.GetMediaCapturePanel`))
      (`/Engine/EditorBlueprintResources/StandardMacros.IsValid` _returnvalue
        (:`Is Valid`
          (`MediaFrameworkCapturePanel.StopCapture` _returnvalue)
          (`MediaFrameworkCapturePanel.EmptyRenderTargetCapture` _returnvalue))))
    (:`then_2`
      (`KismetArrayLibrary.Array_Clear` (`self.SceneCapture2DComponents`))
      (`KismetArrayLibrary.Array_Clear` (`self.RenderTargets`))
      (`KismetArrayLibrary.Array_Clear` (`self.PPMaterials`)))
    (:`then_3`
      (for _index (range (`self.NumSlice`))
        (`|ExecutionSequence`
          (:`then_0`
            (bind _returnvalue_2 (`KismetRenderingLibrary.CreateRenderTarget2D` null (`self.Resx`) (`self.Resy`) "RTF_RGB10A2"))
            (`KismetArrayLibrary.Array_Add` (`self.RenderTargets`) _returnvalue_2))
          (:`then_1`
            (bind _returnvalue_3 (`KismetMaterialLibrary.CreateDynamicMaterialInstance` null (`self.BasePPMaterial`)))
            (`MaterialInstanceDynamic.SetScalarParameterValue` _returnvalue_3 "NearDepth" 0.0)
            (`MaterialInstanceDynamic.SetScalarParameterValue` _returnvalue_3 "FarDepth" (`self.IntervalDistance`))
            (`KismetArrayLibrary.Array_Add` (`self.PPMaterials`) _returnvalue_3))
          (:`then_2`
            (bind _returnvalue_4 (`AddComponent|NODE_AddSceneCaptureComponent2D-2` :`RelativeTransform` (`KismetMathLibrary.MakeTransform` (`KismetMathLibrary.MakeVector` (* _index (`self.IntervalDistance`))))))
            (set `SceneCaptureComponent2D.ProjectionType` "Orthographic" _returnvalue_4)
            (set `SceneCaptureComponent2D.OrthoWidth` (`self.OrthoWidth`) _returnvalue_4)
            (set `SceneCaptureComponent2D.TextureTarget` _returnvalue_2 _returnvalue_4)
            (bind _structout (setmembers `PostProcessSettings` :`StructRef` (`SceneCaptureComponent2D.PostProcessSettings` _returnvalue_4) :`WeightedBlendables` (make `WeightedBlendables` (`|MakeArray` (make `WeightedBlendable` 1.0 _returnvalue_3)))))
            (set `SceneCaptureComponent2D.PostProcessSettings` _structout _returnvalue_4)
            (set `SceneCaptureComponent.CaptureSource` "SCS_FinalToneCurveHDR" _returnvalue_4)
            (`SceneComponent.K2_AttachToComponent` _returnvalue_4 (`self.DefaultSceneRoot`) "None" "KeepRelative" "KeepRelative" "KeepRelative" true)
            (`KismetArrayLibrary.Array_Add` (`self.SceneCapture2DComponents`) _returnvalue_4))
          (:`then_3`
            (bind _output (`|GetArrayItem` (`self.SpoutMediaOutputs`) _index))
            (set `Spout2MediaOutput.OutputSize` (make `IntPoint` (`self.Resx`) (`self.Resy`)) _output)
            (`MediaFrameworkCapturePanel.AddRenderTargetCapture` :`self` _returnvalue :`MediaOutput` _output :`RenderTarget` _returnvalue_2)))))))

(event `self.ReceiveTick`
  (params (DeltaSeconds :type "Float (single-precision)")))

(fn `UserConstructionScript`
  (`|ExecutionSequence`
    (:`then_0`
      (for _array_element (`self.SceneCapture2DComponents`)
        (`ActorComponent.K2_DestroyComponent` _array_element null)))
    (:`then_1`
      (bind _returnvalue (`MediaFrameworkCapturePanelBlueprintLibrary.GetMediaCapturePanel`))
      (`/Engine/EditorBlueprintResources/StandardMacros.IsValid` _returnvalue
        (:`Is Valid`
          (`MediaFrameworkCapturePanel.StopCapture` _returnvalue)
          (`MediaFrameworkCapturePanel.EmptyRenderTargetCapture` _returnvalue))))
    (:`then_2`
      (`KismetArrayLibrary.Array_Clear` (`self.SceneCapture2DComponents`))
      (`KismetArrayLibrary.Array_Clear` (`self.RenderTargets`))
      (`KismetArrayLibrary.Array_Clear` (`self.PPMaterials`)))
    (:`then_3`
      (for _index (range (`self.NumSlice`))
        (`|ExecutionSequence`
          (:`then_0`
            (bind _returnvalue_2 (`KismetRenderingLibrary.CreateRenderTarget2D` null (`self.Resx`) (`self.Resy`) "RTF_RGB10A2"))
            (`KismetArrayLibrary.Array_Add` (`self.RenderTargets`) _returnvalue_2))
          (:`then_1`
            (bind _returnvalue_3 (`KismetMaterialLibrary.CreateDynamicMaterialInstance` null (`self.BasePPMaterial`)))
            (`MaterialInstanceDynamic.SetScalarParameterValue` _returnvalue_3 "NearDepth" 0.0)
            (`MaterialInstanceDynamic.SetScalarParameterValue` _returnvalue_3 "FarDepth" (`self.IntervalDistance`))
            (`KismetArrayLibrary.Array_Add` (`self.PPMaterials`) _returnvalue_3))
          (:`then_2`
            (bind _returnvalue_4 (`AddComponent|NODE_AddSceneCaptureComponent2D-1` :`RelativeTransform` (`KismetMathLibrary.MakeTransform` (`KismetMathLibrary.MakeVector` (* _index (`self.IntervalDistance`))))))
            (set `SceneCaptureComponent2D.ProjectionType` "Orthographic" _returnvalue_4)
            (set `SceneCaptureComponent2D.OrthoWidth` (`self.OrthoWidth`) _returnvalue_4)
            (set `SceneCaptureComponent2D.TextureTarget` _returnvalue_2 _returnvalue_4)
            (bind _structout (setmembers `PostProcessSettings` :`StructRef` (`SceneCaptureComponent2D.PostProcessSettings` _returnvalue_4) :`WeightedBlendables` (make `WeightedBlendables` (`|MakeArray` (make `WeightedBlendable` 1.0 _returnvalue_3)))))
            (set `SceneCaptureComponent2D.PostProcessSettings` _structout _returnvalue_4)
            (set `SceneCaptureComponent.CaptureSource` "SCS_FinalToneCurveHDR" _returnvalue_4)
            (`SceneComponent.K2_AttachToComponent` _returnvalue_4 (`self.DefaultSceneRoot`) "None" "KeepRelative" "KeepRelative" "KeepRelative" true)
            (`KismetArrayLibrary.Array_Add` (`self.SceneCapture2DComponents`) _returnvalue_4))
          (:`then_3`
            (bind _output (`|GetArrayItem` (`self.SpoutMediaOutputs`) _index))
            (set `Spout2MediaOutput.OutputSize` (make `IntPoint` (`self.Resx`) (`self.Resy`)) _output)
            (`MediaFrameworkCapturePanel.AddRenderTargetCapture` :`self` _returnvalue :`MediaOutput` _output :`RenderTarget` _returnvalue_2)))))))