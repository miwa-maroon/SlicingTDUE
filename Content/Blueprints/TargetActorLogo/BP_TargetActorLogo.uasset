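; BP_TargetActorLogo is a logo actor that gives Niagara particle components a box-masked material.
; SetNiagaraDynamicMaterial creates an instance of M_LogoParticleBoxMask, stores it in DynamicMaterials and binds it to the component's MI_LogoBoxMask variable.
; The supplied location and box extent become vector parameters on that instance, so each call gets its own mask.
; The event graph is inactive, and nothing in this Blueprint calls the function.
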(fn `SetNiagaraDynamicMaterial`
  (params (Location :type "LinearColor Structure") (BoxExtent :type "LinearColor Structure") (NS_ParticleComp :type "NiagaraComponent Object Reference"))
  (bind _returnvalue (`KismetMaterialLibrary.CreateDynamicMaterialInstance` "/Game/Materials/M_LogoParticleBoxMask.M_LogoParticleBoxMask"))
  (`KismetArrayLibrary.Array_Add` (`self.DynamicMaterials`) _returnvalue)
  (`NiagaraComponent.SetVariableMaterial` NS_ParticleComp "MI_LogoBoxMask" _returnvalue)
  (`MaterialInstanceDynamic.SetVectorParameterValue` _returnvalue "Location" Location)
  (`MaterialInstanceDynamic.SetVectorParameterValue` _returnvalue "BoxExtent" BoxExtent))

(fn `UserConstructionScript`
  (`parent.UserConstructionScript`))