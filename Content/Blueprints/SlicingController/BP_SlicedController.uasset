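; Controller actor that displays depth slices of a target actor as a tiled grid and outputs them through Spout media capture.
; On BeginPlay it spawns copies in an XZ grid, giving each a thin box at successive Y depths, passed to its dynamic materials.
; It positions and sizes an orthographic scene capture over the grid, then registers RTOutput with the media capture panel.
; Render target creation and assignment nodes are disconnected.
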(event `self.ReceiveBeginPlay`
  (bind _returnvalue (`self.K2_GetActorLocation`))
  (bind _scenecapturecomponent2d (`self.SceneCaptureComponent2D`))
  (bind _spoutmediaoutput (`self.SpoutMediaOutput`))
  (bind _rt_output (`self.RT_Output`))
  (bind _numelementsx (`self.NumElementsX`))
  (bind _index (`self.Index`))
  (for _index_2 (range (`self.NumSlice`))
    (set `self.Index` _index_2)
    (bind _returnvalue_2 (`|SpawnActorFromClass` null (`self.BP_TargetActors`) (`KismetMathLibrary.MakeTransform` _returnvalue) "Undefined" "MultiplyWithRoot" null null))
    (bind _box (`/Game/Blueprints/TargetActorBase/BP_TragetActorsBase.Box` _returnvalue_2))
    (`BoxComponent.SetBoxExtent` _box (`self.BoxExtent`) true)
    (bind (_boxextent_x _boxextent_y _boxextent_z) (`KismetMathLibrary.BreakVector` (`BoxComponent.BoxExtent` _box)))
    (`self.K2_SetActorRelativeLocation` _returnvalue_2 (+ _returnvalue (`KismetMathLibrary.MakeVector` (* (* (mod _index _numelementsx) _boxextent_x) 2.0) 0.0 (* (* (/ _index _numelementsx) _boxextent_z) 2.0))) false false)
    (`|ExecutionSequence`
      (:`then_0`
        (`/Engine/EditorBlueprintResources/StandardMacros.DoOnce` false
          (:`Completed`
            (bind _output_get (set `self.Depth` (* _boxextent_y 2.0)))
            (bind _output_get_2 (set `self.Interval` (/ _output_get (`self.NumSlice`))))
            (set `self.SliceStart` (- _boxextent_y (/ _output_get_2 2.0)))
            (bind _returnvalue_3 (`MediaFrameworkCapturePanelBlueprintLibrary.GetMediaCapturePanel`))
            (`/Engine/EditorBlueprintResources/StandardMacros.IsValid` _returnvalue_3
              (:`Is Valid`
                (`MediaFrameworkCapturePanel.StopCapture` _returnvalue_3)
                (`MediaFrameworkCapturePanel.EmptyRenderTargetCapture` _returnvalue_3))))))
      (:`then_1`
        (`BoxComponent.SetBoxExtent` _box (`KismetMathLibrary.MakeVector` _boxextent_x (/ (`self.Interval`) 2.2) _boxextent_z) true)
        (`SceneComponent.K2_SetRelativeLocation` _box (`KismetMathLibrary.MakeVector` 0.0 (- (`self.SliceStart`) (* (`self.Interval`) (`self.Index`)))) false false)
        (for _array_element (`/Game/Blueprints/TargetActorBase/BP_TragetActorsBase.DynamicMaterials` _returnvalue_2)
          (`MaterialInstanceDynamic.SetVectorParameterValue` _array_element "Location" (`KismetMathLibrary.Conv_VectorToLinearColor` (`SceneComponent.K2_GetComponentLocation` _box)))
          (`MaterialInstanceDynamic.SetVectorParameterValue` _array_element "BoxExtent" (`KismetMathLibrary.Conv_VectorToLinearColor` (`BoxComponent.BoxExtent` _box)))))))
  (`|ExecutionSequence`
    (:`then_1`
      (`SceneComponent.K2_SetWorldLocation` _scenecapturecomponent2d (+ (`self.K2_GetActorLocation`) (`KismetMathLibrary.MakeVector` (* (* _boxextent_x 2.0) (/ (- (`self.NumElementsX`) 1) 2)) 500.0 (* (* _boxextent_z 2.0) (/ (- (`KismetMathLibrary.FCeil` (/ (`KismetMathLibrary.Conv_IntToDouble` (`self.NumSlice`)) (`self.NumElementsX`))) 1) 2)))) false false)
      (set `SceneCaptureComponent2D.OrthoWidth` (* (* _boxextent_x 2.0) (`self.NumElementsX`)) _scenecapturecomponent2d))
    (:`then_2`
      (set `Spout2MediaOutput.OutputSize` (make `IntPoint` (`TextureRenderTarget2D.SizeX` _rt_output) (`TextureRenderTarget2D.SizeY` _rt_output)) _spoutmediaoutput)
      (`MediaFrameworkCapturePanel.AddRenderTargetCapture` :`self` _returnvalue_3 :`MediaOutput` _spoutmediaoutput :`RenderTarget` (`self.RT_Output`)))))

(fn `UserConstructionScript`)