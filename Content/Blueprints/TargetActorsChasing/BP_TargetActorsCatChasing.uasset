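; Target actor that stages a chase between a Cat and a Human component, repeatedly running them across the area.
; A looping timer fires Move, which picks a random start from StartLocations, mirrors it through the origin as the destination and turns both components toward it.
; MoveTimeline then lerps each along that line at a fixed height, with separate tracks for cat and human giving each its own pacing.
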(event `self.ReceiveBeginPlay`
  (bind (_startlocation_x _startlocation_y) (`KismetMathLibrary.BreakVector` (`self.StartLocation`)))
  (`parent.ReceiveBeginPlay`)
  (`SceneComponent.K2_SetRelativeLocation` (`self.Cat`) (`KismetMathLibrary.MakeVector` _startlocation_x _startlocation_y -150.0) false false)
  (`SceneComponent.K2_SetRelativeLocation` (`self.Human`) (`KismetMathLibrary.MakeVector` _startlocation_x _startlocation_y -150.0) false false)
  (`KismetSystemLibrary.K2_SetTimerDelegate` (delegate `Move`) 5.0 true))

(event `Move`
  (bind _startlocation (`self.StartLocation`))
  (bind _destination (`self.Destination`))
  (bind _returnvalue (`KismetMathLibrary.ComposeRotators` (`KismetMathLibrary.FindLookAtRotation` (`self.StartLocation`) (`self.Destination`)) (struct :`Yaw` -90.0)))
  (bind _output_get (set `self.StartLocation` (`|GetArrayItem` (`self.StartLocations`) (`self.RandomIndex`))))
  (set `self.Destination` (* _output_get -1.0))
  (`SceneComponent.K2_SetWorldRotation` (`self.Cat`) _returnvalue false false)
  (`SceneComponent.K2_SetWorldRotation` (`self.Human`) _returnvalue false false)
  (bind (_direction _movehuman _movecat) (`Timeline|MoveTimeline` :!via `PlayFromStart`)
    (:`Update`
      (bind (_returnvalue_x _returnvalue_y) (`KismetMathLibrary.BreakVector` (`KismetMathLibrary.VLerp` _startlocation _destination _movecat)))
      (`SceneComponent.K2_SetRelativeLocation` (`self.Cat`) (`KismetMathLibrary.MakeVector` _returnvalue_x _returnvalue_y -150.0) false false)
      (bind (_returnvalue_x_2 _returnvalue_y_2) (`KismetMathLibrary.BreakVector` (`KismetMathLibrary.VLerp` _startlocation _destination _movehuman)))
      (`SceneComponent.K2_SetRelativeLocation` (`self.Human`) (`KismetMathLibrary.MakeVector` _returnvalue_x_2 _returnvalue_y_2 -150.0) false false))))

(fn `UserConstructionScript`
  (`parent.UserConstructionScript`))